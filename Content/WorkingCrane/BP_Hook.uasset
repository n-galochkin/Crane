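; BP_Hook is a crane hook that captures and releases slingable objects in the working crane simulation.
; On capture it disables physics and lerps to just below the object's calculated hook location with a Timeline.
; It then either hands off to the Slinger_AI worker or slings directly, restoring physics, and a repeat capture call starts unslinging.
; Getters expose the connector and four joints.
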(event `self.hook.OnComponentHit`
  (params (HitComponent :type "PrimitiveComponent Object Reference") (OtherActor :type "Actor Object Reference") (OtherComp :type "PrimitiveComponent Object Reference") (NormalImpulse :type "Vector Structure") (Hit :type "HitResult Structure (by ref)")))

(event `/Game/WorkingCrane/BPI_CraneTool.SetPhysics`
  (params (bEnable :type Boolean))
  (`PrimitiveComponent.SetSimulatePhysics` (`self.hook`) bEnable))

(event `/Game/WorkingCrane/BPI_CraneTool.StartCaptureProccess`
  (bind _hook (`self.hook`))
  (bind (_returnvalue_x _returnvalue_y _returnvalue_z) (`KismetMathLibrary.BreakVector` (`SceneComponent.K2_GetComponentLocation` _hook)))
  (if (and (and (`self.mayCaptureObject`) (`KismetSystemLibrary.IsValid` (`self.capturingObject`))) (not (`self.captured`)))
    (`self.SetPhysics` false)
    (bind _output_get (set `self.lastCapturedObject` (`self.capturingObject`)))
    (bind _newpos (`/Game/Cargo/BP_Container.Calculate Hook Location` _output_get self))
    (bind (_direction _newtrack_2) (`Timeline|Timeline`)
      (:`Update`
        (bind (_returnvalue_x_2 _returnvalue_y_2 _returnvalue_z_2) (`KismetMathLibrary.BreakVector` (`KismetMathLibrary.VLerp` (`KismetMathLibrary.MakeVector` _returnvalue_x _returnvalue_y _returnvalue_z) (`KismetMathLibrary.MakeVector` (.x _newpos) (.y _newpos) (- (.z _newpos) 400.0)) _newtrack_2)))
        (`SceneComponent.K2_SetWorldLocation` _hook (`KismetMathLibrary.MakeVector` _returnvalue_x_2 _returnvalue_y_2 _returnvalue_z_2) false false))
      (:`Finished`
        (if (`self.slingerFlag`)
          (if (`self.NotFirstSling`)
            (`self.Slinger Unpause`)
            (else
              (bind _returnvalue (`GameplayStatics.GetActorOfClass` "/Game/Slinger/AI_Logic/Slinger_AI.Slinger_AI_C"))
              (`/Game/Slinger/AI_Logic/Slinger_AI.startSlinging` _returnvalue)))
          (else
            (`self.SlingingEvent`)))))
    (elif (and (`self.captured`) (`KismetSystemLibrary.IsValid` (`self.lastCapturedObject`)))
      (if (`self.slingerFlag`)
        (`self.Slinger Unpause`)
        (else
          (`/Game/Cargo/BP_Container.Unsling` (`self.lastCapturedObject`) self :!label _label))))))

(event `Unsling Event`
  (set `self.NotFirstSling` true)
  (goto _label))

(event `SlingingEvent`
  (`/Game/Cargo/BP_Container.Slinging` (`self.lastCapturedObject`) self)
  (`self.SetPhysics` true))

(fn `GetConnector`
  (returns (Connector :type "StaticMeshComponent Object Reference"))
  (return (`self.connector`)))

(fn `GetJoints`
  (returns (Joints :type "Array of PrimitiveComponent Object Reference"))
  (return (`|MakeArray` (`self.Joint1`) (`self.Joint2`) (`self.Joint3`) (`self.Joint4`) :!type "PrimitiveComponent Object Reference")))

(fn `UserConstructionScript`)