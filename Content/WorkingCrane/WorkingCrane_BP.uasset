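; Player-controlled crane pawn with rail travel, tower rotation, boom reach, cable winching and swappable capture tools.
; Inputs shift gears on four engine objects, whose velocities AsyncPhysicsTick applies to the actor, AnimBP and cable length, with gear changes shown on the HUD.
; Cable length drives both cable components and physics constraint Z limits.
; Tool switching respawns a BPI_CraneTool actor and binds its joints to cables and constraints by matching component tags.
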(event `self.ReceiveBeginPlay`
  ;[1 1 1] Привязка троссов к крюку при прогрузке уровня
  (`parent.ReceiveBeginPlay`)
  (`self.InitializeJointsPositions`)
  (`self.SetCablesLenght` (`self.cablesLenght`))
  (`self.SwitchTool`))

(event `InputAction|SwitchTool`
  (params (Key :type "Key Structure"))
  ; Смена устройства (кнопка q)
  (:`Pressed`
    (`self.SwitchTool`)))

(event `InputAction|CaptureObject`
  (params (Key :type "Key Structure"))
  ;[1 1 1] Захват Объекта (Кнопка E)
  (:`Pressed`
    (`/Game/WorkingCrane/BPI_CraneTool.StartCaptureProccess` (`self.captureDevice`))))

(event `InputAction|ReachForward`
  (params (Key :type "Key Structure"))
  (bind _bp_enginereach (`self.BP_EngineReach`))
  (bind _gears (`/Game/WorkingCrane/BP_Engine.gears` (`self.BP_EngineReach`)))
  ;[1 1 1] Повышение/понижение передачи вылета стрелы (R - вперед, F - назад)
  (:`Pressed`
    (if (< _gears 2)
      (bind _result (`/Engine/EditorBlueprintResources/StandardMacros.IncrementInt` _gears)
        (:`  `
          (`KismetSystemLibrary.PrintText` (`KismetTextLibrary.Conv_IntToText` _result))
          (if true :!label _label
            (`/Game/WorkingCrane/BP_Engine.GearChanging` _bp_enginereach)
            (`self.updateHUD` 2 (`KismetTextLibrary.Conv_DoubleToText` (`KismetMathLibrary.Conv_IntToDouble` (`/Game/WorkingCrane/BP_Engine.gears` _bp_enginereach)) "HalfToEven"))))))))

(event `InputAction|LiftCables`
  (params (Key :type "Key Structure"))
  (bind _bp_enginecables (`self.BP_EngineCables`))
  (bind _gears (`/Game/WorkingCrane/BP_Engine.gears` (`self.BP_EngineCables`)))
  ;[1 1 1] Повышение/понижение передачи изменения длины тросса (Z - Разматывание, X - Сматиывание)
  (:`Pressed`
    (if (< _gears 3)
      (bind _result (`/Engine/EditorBlueprintResources/StandardMacros.IncrementInt` _gears)
        (:`  `
          (if true :!label _label_2
            (`/Game/WorkingCrane/BP_Engine.GearChanging` _bp_enginecables)
            (`self.updateHUD` 3 (`KismetTextLibrary.Conv_IntToText` (`/Game/WorkingCrane/BP_Engine.gears` _bp_enginecables)))))))))

(event `InputAction|ReachBackward`
  (params (Key :type "Key Structure"))
  (bind _gears (`/Game/WorkingCrane/BP_Engine.gears` (`self.BP_EngineReach`)))
  ;[1 1 1] Повышение/понижение передачи вылета стрелы (R - вперед, F - назад)
  (:`Pressed`
    (if (> _gears -2)
      (bind _result (`/Engine/EditorBlueprintResources/StandardMacros.DecrementInt` _gears)
        (:`  `
          (`KismetSystemLibrary.PrintText` (`KismetTextLibrary.Conv_IntToText` _result))
          (goto _label))))))

(event `InputAction|LowerCables`
  (params (Key :type "Key Structure"))
  (bind _gears (`/Game/WorkingCrane/BP_Engine.gears` (`self.BP_EngineCables`)))
  ;[1 1 1] Повышение/понижение передачи изменения длины тросса (Z - Разматывание, X - Сматиывание)
  (:`Pressed`
    (if (> _gears -3)
      (bind _result (`/Engine/EditorBlueprintResources/StandardMacros.DecrementInt` _gears)
        (:`  `
          (goto _label_2))))))

(event `InputAction|UpshiftRails`
  (params (Key :type "Key Structure"))
  (bind _bp_enginemove (`self.BP_EngineMove`))
  (bind _gears (`/Game/WorkingCrane/BP_Engine.gears` (`self.BP_EngineMove`)))
  ;[1 1 1] Повышение/понижение передачи движения крана (W - вперед / S - назад)
  (:`Pressed`
    (if (< _gears 2)
      (bind _result (`/Engine/EditorBlueprintResources/StandardMacros.IncrementInt` _gears)
        (:`  `
          (if true :!label _label_3
            (`/Game/WorkingCrane/BP_Engine.GearChanging` _bp_enginemove)
            (`self.updateHUD` 0 (`KismetTextLibrary.Conv_IntToText` (`/Game/WorkingCrane/BP_Engine.gears` _bp_enginemove)))))))))

(event `InputAction|RotateTowerRight`
  (params (Key :type "Key Structure"))
  (bind _bp_enginerotate (`self.BP_EngineRotate`))
  (bind _gears (`/Game/WorkingCrane/BP_Engine.gears` (`self.BP_EngineRotate`)))
  ;[1 1 1] Повышение/понижение передачи поворота башни (A - влево, D - право, left arrow, right arrow)
  (:`Pressed`
    (if (< _gears 2)
      (bind _result (`/Engine/EditorBlueprintResources/StandardMacros.IncrementInt` _gears)
        (:`  `
          (if true :!label _label_4
            (`/Game/WorkingCrane/BP_Engine.GearChanging` _bp_enginerotate)
            (`self.updateHUD` 1 (`KismetTextLibrary.Conv_IntToText` (`/Game/WorkingCrane/BP_Engine.gears` _bp_enginerotate)))))))))

(event `InputAction|DownshiftRails`
  (params (Key :type "Key Structure"))
  (bind _gears (`/Game/WorkingCrane/BP_Engine.gears` (`self.BP_EngineMove`)))
  ;[1 1 1] Повышение/понижение передачи движения крана (W - вперед / S - назад)
  (:`Pressed`
    (if (> _gears -2)
      (bind _result (`/Engine/EditorBlueprintResources/StandardMacros.DecrementInt` _gears)
        (:`  `
          (goto _label_3))))))

(event `InputAction|RotateTowerLeft`
  (params (Key :type "Key Structure"))
  (bind _gears (`/Game/WorkingCrane/BP_Engine.gears` (`self.BP_EngineRotate`)))
  ;[1 1 1] Повышение/понижение передачи поворота башни (A - влево, D - право, left arrow, right arrow)
  (:`Pressed`
    (if (> _gears -2)
      (bind _result (`/Engine/EditorBlueprintResources/StandardMacros.DecrementInt` _gears)
        (:`  `
          (goto _label_4))))))

(event `InputAxis|MouseUpDown`
  (params (AxisValue :type "Float (single-precision)"))
  ;[1 1 1] Вращение головой
  (`self.AddControllerPitchInput` AxisValue))

(event `self.ReceiveAsyncPhysicsTick`
  (params (DeltaSeconds :type "Float (single-precision)") (SimSeconds :type "Float (single-precision)"))
  (bind _bp_enginecables (`self.BP_EngineCables`))
  (bind _joint1 (`self.Joint1`))
  (bind (_returnvalue_roll _returnvalue_pitch _returnvalue_yaw) (`KismetMathLibrary.BreakRotator` (`SceneComponent.K2_GetComponentRotation` _joint1)))
  (bind _gears (`/Game/WorkingCrane/BP_Engine.gears` _bp_enginecables))
  ;[1 1 1] Перемещение крана
  (`|ExecutionSequence`
    (:`then_0`
      (bind _outputvel (`/Game/WorkingCrane/BP_Engine.CalculateOutputVelocity` (`self.BP_EngineMove`) SimSeconds))
      (`self.K2_AddActorWorldOffset` (* (`self.GetActorForwardVector`) _outputvel)))
    (:`then_1`
      ;[1 1 1] Поворот башни крана
      (bind _outputvel_2 (`/Game/WorkingCrane/BP_Engine.CalculateOutputVelocity` (`self.BP_EngineRotate`) SimSeconds))
      (bind _asabp_working_crane (cast `/Game/WorkingCrane/Crane/ABP_WorkingCrane` (`SkeletalMeshComponent.GetAnimInstance` (`self.SkeletalMesh`))))
      (bind (_rotatetower_roll _rotatetower_pitch _rotatetower_yaw) (`KismetMathLibrary.BreakRotator` (`/Game/WorkingCrane/Crane/ABP_WorkingCrane.rotateTower` _asabp_working_crane)))
      (set `/Game/WorkingCrane/Crane/ABP_WorkingCrane.rotateTower` (`KismetMathLibrary.MakeRotator` 0.0 0.0 (+ _outputvel_2 _rotatetower_yaw)) _asabp_working_crane))
    (:`then_2`
      ;[1 1 1] Изменение длины троссов
      (bind _outputvel_3 (`/Game/WorkingCrane/BP_Engine.CalculateOutputVelocity` _bp_enginecables SimSeconds))
      (bind _returnvalue (`PhysicsConstraintComponent.GetConstraint` (`self.PhysicsConstraint1`)))
      (bind (_xmotion _ymotion _zmotion _limit) (`ConstraintInstanceBlueprintLibrary.GetLinearLimits` _returnvalue))
      (bind _connector (`/Game/WorkingCrane/BPI_CraneTool.GetConnector` (`self.captureDevice`)))
      (bind (_returnvalue_x _returnvalue_y _returnvalue_z) (`KismetMathLibrary.BreakVector` (`SceneComponent.K2_GetComponentLocation` _connector)))
      (if (not (or (and (<= (- _returnvalue_z 15.0) 0.0) (> _gears 0)) (and (<= _limit (`self.minLenght`)) (< _gears 0))))
        (`self.addCablesLenght` (/ _outputvel_3 1.0))))
    (:`then_3`
      ;[1 1 1] Вылет стрелы
      (bind _outputvel_4 (`/Game/WorkingCrane/BP_Engine.CalculateOutputVelocity` (`self.BP_EngineReach`) SimSeconds))
      (bind _asabp_working_crane_2 (cast `/Game/WorkingCrane/Crane/ABP_WorkingCrane` (`SkeletalMeshComponent.GetAnimInstance` (`self.SkeletalMesh`))))
      (set `/Game/WorkingCrane/Crane/ABP_WorkingCrane.reachSpeed` (+ (`/Game/WorkingCrane/Crane/ABP_WorkingCrane.reachSpeed` _asabp_working_crane_2) _outputvel_4) _asabp_working_crane_2)
      ;[1 1 1] При вылете стрелы изменяется вращение сокета по X сбрасываем значение чтобы constraint смотрел строго вниз
      (`SceneComponent.K2_SetWorldRotation` _joint1 (`KismetMathLibrary.MakeRotator` 0.0 _returnvalue_pitch _returnvalue_yaw) false false)
      (`SceneComponent.K2_SetWorldRotation` (`self.Joint2`) (`KismetMathLibrary.MakeRotator` 0.0 _returnvalue_pitch _returnvalue_yaw) false false)
      (`SceneComponent.K2_SetWorldRotation` (`self.Joint3`) (`KismetMathLibrary.MakeRotator` 0.0 _returnvalue_pitch _returnvalue_yaw) false false)
      (`SceneComponent.K2_SetWorldRotation` (`self.Joint4`) (`KismetMathLibrary.MakeRotator` 0.0 _returnvalue_pitch _returnvalue_yaw) false false))))

(event `InputAxis|MouseRightLeft`
  (params (AxisValue :type "Float (single-precision)"))
  ;[1 1 1] Вращение головой
  (`self.AddControllerYawInput` AxisValue))

(fn `addCablesLenght`
  (params (DeltaLenght :type "Float (double-precision)"))
  (`self.SetCablesLenght` (+ DeltaLenght (`self.cablesLenght`))))

(fn `AttachCableEndToJoint`
  (params (DeviceJoint :type "SceneComponent Object Reference") (Tag :type Name))
  (locals (FoundCable :type "CableComponent Object Reference"))
  (bind _output_get (set `local.FoundCable` (`self.FindComponentByTag` "/Script/CableComponent.CableComponent" Tag)))
  (`CableComponent.SetAttachEndToComponent` _output_get DeviceJoint "None")
  (set `CableComponent.EndLocation` (0.0 0.0 0.0) _output_get))

(fn `AttachDevice`
  (params (CaptureDevice :type "/Game/WorkingCrane/BPI_CraneTool Interface"))
  (bind _output_get (set `self.captureDevice` CaptureDevice))
  (bind _joints (`/Game/WorkingCrane/BPI_CraneTool.GetJoints` _output_get))
  (`/Game/WorkingCrane/BPI_CraneTool.SetPhysics` _output_get false)
  (for _array_element _joints
    (bind _componenttags (`ActorComponent.ComponentTags` _array_element))
    (if (`KismetArrayLibrary.Array_IsNotEmpty` _componenttags)
      (bind _output (`|GetArrayItem` _componenttags))
      (`self.AttachCableEndToJoint` _array_element _output)
      (`self.AttachJointsByPhysics` _array_element _output)
      (else
        (`KismetSystemLibrary.PrintString` (`KismetStringLibrary.Concat_StrStr` (`KismetSystemLibrary.GetDisplayName` _array_element) "No Cable Tag to attach!") true true (struct :`R` 1.0 :`G` 0.039492 :`A` 1.0)))))
  (`/Game/WorkingCrane/BPI_CraneTool.SetPhysics` _output_get true))

(fn `AttachJointsByPhysics`
  (params (DeviceJoint :type "PrimitiveComponent Object Reference") (Tag :type Name))
  (`PhysicsConstraintComponent.SetConstrainedComponents` (`self.FindComponentByTag` "/Script/Engine.PhysicsConstraintComponent" Tag) (`self.FindComponentByTag` "/Script/Engine.StaticMeshComponent" Tag) "None" DeviceJoint "None"))

(fn `CalculateVelocity`
  (params (k :type "Float (double-precision)") (colVelocity :type "Float (double-precision)") (t1 :type "Float (double-precision)") (t2 :type "Float (double-precision)") (elapsTime :type "Float (double-precision)"))
  (returns (outVel :type "Float (double-precision)"))
  (return (+ colVelocity (* k (+ (- 1.0 (* (/ t1 (- t1 t2)) (`KismetMathLibrary.Exp` (/ (* -1.0 elapsTime) t1)))) (* (/ t2 (- t1 t2)) (`KismetMathLibrary.Exp` (/ (* -1.0 elapsTime) t2))))))))

(fn `CalculateVelocity_0`
  (params (deltaTime :type "Float (double-precision)"))
  (returns (outVel :type "Float (double-precision)"))
  (set `self.timeElapsed` (+ (`self.timeElapsed`) deltaTime))
  (bind _output_get (set `self.outputVelocityRails` (+ (`self.colectedVelocityRails`) (* (`self.k`) (+ (- 1.0 (* (/ (`self.t1`) (- (`self.t1`) (`self.t2`))) (`KismetMathLibrary.Exp` (/ (* -1.0 (`self.timeElapsed`)) (`self.t1`))))) (* (/ (`self.t2`) (- (`self.t1`) (`self.t2`))) (`KismetMathLibrary.Exp` (/ (* -1.0 (`self.timeElapsed`)) (`self.t2`)))))))))
  (return _output_get))

(fn `InitializeJointsPositions`
  (bind _joint1 (`self.Joint1`))
  (bind (_returnvalue_roll _returnvalue_pitch _returnvalue_yaw) (`KismetMathLibrary.BreakRotator` (`SceneComponent.K2_GetComponentRotation` _joint1)))
  (`SceneComponent.K2_SetWorldRotation` _joint1 (`KismetMathLibrary.MakeRotator` 0.0 _returnvalue_pitch _returnvalue_yaw) false false)
  (`SceneComponent.K2_SetWorldRotation` (`self.Joint2`) (`KismetMathLibrary.MakeRotator` 0.0 _returnvalue_pitch _returnvalue_yaw) false false)
  (`SceneComponent.K2_SetWorldRotation` (`self.Joint3`) (`KismetMathLibrary.MakeRotator` 0.0 _returnvalue_pitch _returnvalue_yaw) false false)
  (`SceneComponent.K2_SetWorldRotation` (`self.Joint4`) (`KismetMathLibrary.MakeRotator` 0.0 _returnvalue_pitch _returnvalue_yaw) false false))

(fn `movePhysicsConstraintToMidleOfRopes`
  (params (HooksWorldLoc :type "Vector Structure") (Z :type "Float (double-precision)"))
  (bind _physicsconstraint3 (`self.PhysicsConstraint3`))
  (bind _physicsconstraint4 (`self.PhysicsConstraint4`))
  (bind _physicsconstraint2 (`self.PhysicsConstraint2`))
  (bind _physicsconstraint1 (`self.PhysicsConstraint1`))
  (bind _physicsconstraint1_2 (`self.PhysicsConstraint1`))
  (bind (_returnvalue_x _returnvalue_y) (`KismetMathLibrary.BreakVector` (`SceneComponent.K2_GetComponentLocation` _physicsconstraint4)))
  (bind (_returnvalue_x_2 _returnvalue_y_2 _returnvalue_z) (`KismetMathLibrary.BreakVector` (`SceneComponent.K2_GetComponentLocation` (`self.PhysicsConstraint1`))))
  (bind (_returnvalue_x_3 _returnvalue_y_3) (`KismetMathLibrary.BreakVector` (`SceneComponent.K2_GetComponentLocation` _physicsconstraint2)))
  (bind (_returnvalue_x_4 _returnvalue_y_4) (`KismetMathLibrary.BreakVector` (`SceneComponent.K2_GetComponentLocation` _physicsconstraint3)))
  (bind (_returnvalue_x_5 _returnvalue_y_5) (`KismetMathLibrary.BreakVector` (`SceneComponent.K2_GetComponentLocation` _physicsconstraint1)))
  (bind _returnvalue (- _returnvalue_z Z))
  (`SceneComponent.K2_SetWorldLocation` _physicsconstraint1 (`KismetMathLibrary.MakeVector` _returnvalue_x_5 _returnvalue_y_5 _returnvalue) false false)
  (`SceneComponent.K2_SetWorldLocation` _physicsconstraint2 (`KismetMathLibrary.MakeVector` _returnvalue_x_3 _returnvalue_y_3 _returnvalue) false false)
  (`SceneComponent.K2_SetWorldLocation` _physicsconstraint3 (`KismetMathLibrary.MakeVector` _returnvalue_x_4 _returnvalue_y_4 _returnvalue) false false)
  (`SceneComponent.K2_SetWorldLocation` _physicsconstraint4 (`KismetMathLibrary.MakeVector` _returnvalue_x _returnvalue_y _returnvalue) false false)
  (`SceneComponent.K2_SetRelativeLocation` _physicsconstraint1_2 (* (`SceneComponent.RelativeLocation` _physicsconstraint1_2) 2.0) false false))

(fn `ReleaseCargo`
  (params (captureDevice :type "/Game/WorkingCrane/BP_Hook Object Reference")))

(fn `SetCablesLenght`
  (params (newLenght :type "Float (double-precision)"))
  (set `self.cablesLenght` newLenght)
  (for _array_element (`self.K2_GetComponentsByClass` "/Script/CableComponent.CableComponent")
    (set `CableComponent.CableLength` (`self.cablesLenght`) _array_element))
  (for _array_element_2 (`self.K2_GetComponentsByClass` "/Script/Engine.PhysicsConstraintComponent")
    (`PhysicsConstraintComponent.SetLinearZLimit` _array_element_2 "LCM_Limited" (+ (`self.cablesLenght`) 100.0))))

(fn `SetTime`
  (params (T1 :type "Float (double-precision)") (T2 :type "Float (double-precision)"))
  (set `self.t1` T1)
  (set `self.t2` T2))

(fn `SwitchTool`
  (locals (ToolIndex :type Integer :default 1))
  (bind _capturedevice (`self.captureDevice`))
  (bind _toolsclasses (`self.ToolsClasses`))
  (bind _asactor (cast `Actor` (`KismetSystemLibrary.Conv_InterfaceToObject` _capturedevice) :!pure true))
  (`|ExecutionSequence`
    (:`then_0`
      ; Смена индекса класса и удаление старого инструмента
      (if (`KismetSystemLibrary.IsValidInterface` _capturedevice)
        (bind _result (`/Engine/EditorBlueprintResources/StandardMacros.IncrementInt` (`KismetArrayLibrary.Array_Find` _toolsclasses (`GameplayStatics.GetObjectClass` _asactor)))
          (:`  `
            (set `local.ToolIndex` (mod _result (`KismetArrayLibrary.Array_Length` _toolsclasses)))
            (`self.K2_DestroyActor` _asactor)))))
    (:`then_1`
      ; Спавн нового инструмента и прикрепление его к крану
      (bind _returnvalue (`|SpawnActorFromClass` (`|GetArrayItem` (`self.ToolsClasses`) (`local.ToolIndex`)) (`KismetMathLibrary.MakeTransform` (+ (`SceneComponent.K2_GetComponentLocation` (`self.CenterOfJoints`)) (`KismetMathLibrary.MakeVector` 0.0 0.0 (* -1.0 (`self.cablesLenght`)))) (`self.K2_GetActorRotation`)) "AlwaysSpawn" "MultiplyWithRoot" self null))
      (bind _asbpi_crane_tool (cast `/Game/WorkingCrane/BPI_CraneTool` _returnvalue))
      (`self.AttachDevice` _asbpi_crane_tool))))

(fn `updateHUD`
  (params (EngineType :type Integer) (text :type Text))
  (bind _asbp_hud (cast `/Game/BP_HUD` (`PlayerController.GetHUD` (`GameplayStatics.GetPlayerController` 0))))
  (`/Game/WorkingCrane/WBP_CraneUserHints.Update Text` (`/Game/BP_HUD.UI_ref` _asbp_hud) EngineType text))

(fn `UserConstructionScript`)