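; BP_Engine models an engine's velocity response to gear and power, apparently for the working crane.
; GearChanging stores the current velocity, derives the step K from gear, power and that velocity, and restarts the timer.
; CalculateOutputVelocity advances time and evaluates an analytic second-order lag step response from the stored velocity, using two exponential time constants.
; Gear zero selects braking time constants; other gears use starting ones.
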(fn CalculateVelocity
  (params (k :type Float%20%28double-precision%29) (colVelocity :type Float%20%28double-precision%29) (t1 :type Float%20%28double-precision%29) (t2 :type Float%20%28double-precision%29) (elapsTime :type Float%20%28double-precision%29))
  (return (+ colVelocity (* k (+ (- 1.0 (* (/ t1 (- t1 t2)) (Class|KismetMathLibrary|Exp (/ (* -1.0 elapsTime) t1)))) (* (/ t2 (- t1 t2)) (Class|KismetMathLibrary|Exp (/ (* -1.0 elapsTime) t2))))))))

(fn GearChanging
  (bind _outputvelocity (Variables|Default|GetoutputVelocity))
  (Variables|Default|SetcollectedVeloctiy _outputvelocity)
  (Variables|Default|Setk (|((gearNow*p)-outputVel) (Math|Conversions|ToFloat(Integer) (Variables|Default|Getgears)) (Variables|Default|Getpower) _outputvelocity))
  (Variables|Default|SettimeElapsed 0.0))

(fn SetTime
  (params (T1 :type Float%20%28double-precision%29) (T2 :type Float%20%28double-precision%29))
  (Variables|Default|Sett1 T1)
  (Variables|Default|Sett2 T2))

(fn CalculateOutputVelocity
  (params (deltaT :type Float%20%28double-precision%29))
  (if (== (Variables|Default|Getgears) 0)
    (CallFunction|SetTime (Variables|Default|GettimeOfBreaking1) (Variables|Default|GettimeOfBreaking2))
    (else
      (CallFunction|SetTime (Variables|Default|GettimeOfStarting1) (Variables|Default|GettimeOfStarting2))))
  (bind _output_get (Variables|Default|SettimeElapsed (+ (Variables|Default|GettimeElapsed) deltaT)))
  (bind _outvel (CallFunction|CalculateVelocity (Variables|Default|Getk) (Variables|Default|GetcollectedVeloctiy) (Variables|Default|Gett1) (Variables|Default|Gett2) _output_get))
  (bind _output_get_2 (Variables|Default|SetoutputVelocity _outvel))
  (return _output_get_2))