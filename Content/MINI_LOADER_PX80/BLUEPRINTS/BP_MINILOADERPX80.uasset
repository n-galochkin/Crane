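; Player-drivable PX80 mini loader on Chaos vehicle movement that scoops and dumps debris.
; Tick feeds driving input, cameras, steering wheel, speed-driven sound, smoke and reverse lights, plus optional fuel drain that cuts throttle when empty.
; Held inputs step clamped arm and spade rotation values.
; Trigger overlaps move debris from BP_LoadDebris to BP_DumpDebris, dumping only with the arm raised and spade tilted.
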(event `InputAction|Lights`
  (params (Key :type "Key Structure"))
  (:`Pressed`
    (`/Engine/EditorBlueprintResources/StandardMacros.FlipFlop`
      (:`A`
        (`SceneComponent.SetVisibility` (`self.FLightRight`) true false)
        (`SceneComponent.SetVisibility` (`self.FLightLeft`) true false)
        (`SceneComponent.SetVisibility` (`self.FrontLightGlow`) true false))
      (:`B`
        (`SceneComponent.SetVisibility` (`self.FLightLeft`) false false)
        (`SceneComponent.SetVisibility` (`self.FLightRight`) false false)
        (`SceneComponent.SetVisibility` (`self.FrontLightGlow`) false false)))))

(event `Key|SpaceBar`
  (params (Key :type "Key Structure"))
  (:`Pressed`
    (`self.StopLights` :!label _label))
  (:`Released`
    (goto _label :!via `InputPin`)))

(event `InputAction|Handbrake`
  (params (Key :type "Key Structure"))
  (:`Pressed`
    (goto _label))
  (:`Released`
    (goto _label :!via `InputPin`)))

(event `InputAction|SwitchCamera`
  (params (Key :type "Key Structure"))
  (bind _maincamera (`self.MainCamera`))
  (bind _interiorcamera (`self.InteriorCamera`))
  (:`Pressed`
    (`/Engine/EditorBlueprintResources/StandardMacros.FlipFlop`
      (:`A`
        (`ActorComponent.Activate` _interiorcamera false)
        (`ActorComponent.Deactivate` _maincamera))
      (:`B`
        (`ActorComponent.Activate` _maincamera false)
        (`ActorComponent.Deactivate` _interiorcamera)))))

(event `Key|MouseScrollDown`
  (params (Key :type "Key Structure"))
  (bind _mainspringarm (`self.MainSpringArm`))
  (:`Pressed`
    (set `SpringArmComponent.TargetArmLength` (+ (`KismetMathLibrary.FClamp` (`SpringArmComponent.TargetArmLength` _mainspringarm) 400.0 2000.0) 20.0) _mainspringarm)))

(event `Key|MouseScrollUp`
  (params (Key :type "Key Structure"))
  (bind _mainspringarm (`self.MainSpringArm`))
  (:`Pressed`
    (set `SpringArmComponent.TargetArmLength` (- (`KismetMathLibrary.FClamp` (`SpringArmComponent.TargetArmLength` _mainspringarm) 400.0 2000.0) 20.0) _mainspringarm)))

(event `self.ReceiveBeginPlay`
  ;[0.3125 0 0 1 40] BEGIN PLAY EVENTS
  (`self.ATTENTION LIGHT`)
  (bind _returnvalue (`|CreateWidget` "/Game/MINI_LOADER_PX80/Widget/W_LOADERPX80_HUD.W_LOADERPX80_HUD_C"))
  (`UserWidget.AddToViewport` _returnvalue 0)
  ;;[1 0 0.4755] DELETE THIS SECTION
  (bind _returnvalue_2 (`|CreateWidget` "/Game/MINI_LOADER_PX80/Widget/W_HUDLOGO.W_HUDLOGO_C"))
  (`UserWidget.AddToViewport` _returnvalue_2 0))

(event `self.DumpTrigger.OnComponentBeginOverlap`
  (params (OverlappedComponent :type "PrimitiveComponent Object Reference") (OtherActor :type "Actor Object Reference") (OtherComp :type "PrimitiveComponent Object Reference") (OtherBodyIndex :type Integer) (bFromSweep :type Boolean) (SweepResult :type "HitResult Structure (by ref)"))
  (bind _dustparticle (`self.DustParticle`))
  (bind _asbp_dump_debris (cast `/Game/MINI_LOADER_PX80/BLUEPRINTS/BP_DumpDebris` OtherActor))
  (if (`self.DebrisLoaded?`)
    (`/Engine/EditorBlueprintResources/StandardMacros.DoOnce` false :!label _label_2
      (:`Completed`
        (if (> (`self.FrontArmRotating`) 35.0)
          (if (< (`self.SpadeRotating`) -30.0)
            (`SceneComponent.SetVisibility` (`self.SpadeDebris`) false false)
            (set `/Game/MINI_LOADER_PX80/BLUEPRINTS/BP_DumpDebris.DumperDebrisValue` (+ (`/Game/MINI_LOADER_PX80/BLUEPRINTS/BP_DumpDebris.DumperDebrisValue` _asbp_dump_debris) (`/Game/MINI_LOADER_PX80/BLUEPRINTS/BP_DumpDebris.DumperDebrisLoadValue` _asbp_dump_debris)) _asbp_dump_debris)
            (set `self.DebrisLoaded?` false)
            (`SceneComponent.SetVisibility` _dustparticle true false)
            (`KismetSystemLibrary.Delay` 2.0)
            (`SceneComponent.SetVisibility` _dustparticle false false)))))))

(event `self.LoadTrigger.OnComponentEndOverlap`
  (params (OverlappedComponent :type "PrimitiveComponent Object Reference") (OtherActor :type "Actor Object Reference") (OtherComp :type "PrimitiveComponent Object Reference") (OtherBodyIndex :type Integer))
  (cast `/Game/MINI_LOADER_PX80/BLUEPRINTS/BP_LoadDebris` OtherActor)
  (goto _label_3 :!via `Reset`))

(event `self.LoadTrigger.OnComponentBeginOverlap`
  (params (OverlappedComponent :type "PrimitiveComponent Object Reference") (OtherActor :type "Actor Object Reference") (OtherComp :type "PrimitiveComponent Object Reference") (OtherBodyIndex :type Integer) (bFromSweep :type Boolean) (SweepResult :type "HitResult Structure (by ref)"))
  (bind _asbp_load_debris (cast `/Game/MINI_LOADER_PX80/BLUEPRINTS/BP_LoadDebris` OtherActor))
  (if (not (`self.DebrisLoaded?`))
    (`/Engine/EditorBlueprintResources/StandardMacros.DoOnce` false :!label _label_3
      (:`Completed`
        (`SceneComponent.SetVisibility` (`self.SpadeDebris`) true false)
        (set `/Game/MINI_LOADER_PX80/BLUEPRINTS/BP_LoadDebris.DebrisValue` (- (`/Game/MINI_LOADER_PX80/BLUEPRINTS/BP_LoadDebris.DebrisValue` _asbp_load_debris) 0.2) _asbp_load_debris)
        (set `self.DebrisLoaded?` true)))))

(event `self.DumpTrigger.OnComponentEndOverlap`
  (params (OverlappedComponent :type "PrimitiveComponent Object Reference") (OtherActor :type "Actor Object Reference") (OtherComp :type "PrimitiveComponent Object Reference") (OtherBodyIndex :type Integer))
  (cast `/Game/MINI_LOADER_PX80/BLUEPRINTS/BP_DumpDebris` OtherActor)
  (goto _label_2 :!via `Reset`))

(event `self.ReceiveTick`
  (params (DeltaSeconds :type "Float (single-precision)"))
  (bind _spaderotating (`self.SpadeRotating`))
  (bind _frontarmrotating (`self.FrontArmRotating`))
  (bind _maxspaderotating (`self.MaxSpadeRotating`))
  (bind _maxarmrotating (`self.MaxArmRotating`))
  ;[0.06128 1 0 1 40] EVENT TICK
  (`self.Camera_Input`)
  (`self.InteriorCamera_Input`)
  (`self.SteeringWheelRotation` DeltaSeconds)
  (`|ExecutionSequence`
    (:`then_0`
      (`self.FuelSystem`)
      (if (`self.FuelFinish?`)
        (`self.FuelFinish`)
        (else
          (`self.Vehicle_Inputs`)
          (`self.Car_Sound`)
          (`self.ReverseLights`)
          (`self.BackSmoke`))))
    (:`then_1`
      (`|ExecutionSequence`
        (:`then_0`
          (if (`self.FrontArmUp?`)
            (bind _result (`/Engine/EditorBlueprintResources/StandardMacros.IncrementFloat` _frontarmrotating)
              (:`  `
                (set `self.FrontArmRotating` (`KismetMathLibrary.FClamp` _result 0.0 _maxarmrotating))))))
        (:`then_1`
          (if (`self.FrontArmDown`)
            (bind _result_2 (`/Engine/EditorBlueprintResources/StandardMacros.DecrementFloat` _frontarmrotating)
              (:`  `
                (set `self.FrontArmRotating` (`KismetMathLibrary.FClamp` _result_2 0.0 _maxarmrotating))))))
        (:`then_2`
          (if (`self.FrontSpadeUp?`)
            (bind _result_3 (`/Engine/EditorBlueprintResources/StandardMacros.IncrementFloat` _spaderotating)
              (:`  `
                (set `self.SpadeRotating` (`KismetMathLibrary.FClamp` _result_3 _maxspaderotating 0.0))))))
        (:`then_3`
          (if (`self.FrontSpadeDown`)
            (bind _result_4 (`/Engine/EditorBlueprintResources/StandardMacros.DecrementFloat` _spaderotating)
              (:`  `
                (set `self.SpadeRotating` (`KismetMathLibrary.FClamp` _result_4 _maxspaderotating 0.0))))))))))

(event `InputAction|FrontArmUp`
  (params (Key :type "Key Structure"))
  (bind _s_hydrolic (`self.S_Hydrolic`))
  ;[0.06128 1 0 1 40] EVENT TICK
  (:`Pressed`
    (set `self.FrontArmUp?` true)
    (`AudioComponent.Play` _s_hydrolic 0.0 :!label _label_4))
  (:`Released`
    (set `self.FrontArmUp?` false)
    (`AudioComponent.Stop` _s_hydrolic :!label _label_5)))

(event `InputAction|FrontArmDown`
  (params (Key :type "Key Structure"))
  ;[0.06128 1 0 1 40] EVENT TICK
  (:`Pressed`
    (set `self.FrontArmDown` true)
    (goto _label_4))
  (:`Released`
    (set `self.FrontArmDown` false)
    (goto _label_5)))

(event `InputAction|FrontSpadeUp`
  (params (Key :type "Key Structure"))
  (bind _s_hydrolic (`self.S_Hydrolic`))
  ;[0.06128 1 0 1 40] EVENT TICK
  (:`Pressed`
    (set `self.FrontSpadeUp?` true)
    (`AudioComponent.Play` _s_hydrolic 0.0 :!label _label_6))
  (:`Released`
    (set `self.FrontSpadeUp?` false)
    (`AudioComponent.Stop` _s_hydrolic :!label _label_7)))

(event `InputAction|FrontSpadeDown`
  (params (Key :type "Key Structure"))
  ;[0.06128 1 0 1 40] EVENT TICK
  (:`Pressed`
    (set `self.FrontSpadeDown` true)
    (goto _label_6))
  (:`Released`
    (set `self.FrontSpadeDown` false)
    (goto _label_7)))

(event `InputAction|Handbrake`
  (params (Key :type "Key Structure"))
  (bind _vehiclemovementcomponent (`self.VehicleMovementComponent`))
  ;[0 0 0 1 30] HANDBRAKE
  (:`Pressed`
    (`ChaosVehicleMovementComponent.SetHandbrakeInput` _vehiclemovementcomponent true)
    (set `self.HandBrake?` true))
  (:`Released`
    (`ChaosVehicleMovementComponent.SetHandbrakeInput` _vehiclemovementcomponent false)
    (set `self.HandBrake?` false)))

(event `ATTENTION LIGHT`
  (bind _attentionlight (`self.AttentionLight`))
  ;[0 0 0 1 30] ATTENTION LIGHT VISIBILITY
  (if (`self.AttentionLightVisibility?`)
    (`SceneComponent.SetVisibility` _attentionlight true false)
    (else
      (`SceneComponent.SetVisibility` _attentionlight false false))))

(event `InputAction|FlipCar`
  (params (Key :type "Key Structure"))
  ;[0 0 0 1 30] FLIP CAR
  (:`Pressed`
    (`self.FlipCar`)))

(event `Key|Tab`
  (params (Key :type "Key Structure"))
  ;[0 0 0 1 30] CONTROLS PANEL - DELETE THIS SECTION
  (:`Pressed`
    (`/Engine/EditorBlueprintResources/StandardMacros.FlipFlop`
      (:`A`
        (bind _returnvalue (`|CreateWidget` "/Game/MINI_LOADER_PX80/Widget/W_CONTROLS_INGAME.W_CONTROLS_INGAME_C" (`GameplayStatics.GetPlayerController` 0)))
        (`UserWidget.AddToViewport` _returnvalue 0))
      (:`B`
        (`Widget.RemoveFromParent` _returnvalue)))))

(fn `BackSmoke`
  (bind _smoke (`self.SMOKE`))
  ;[0 0 0] BACK SMOKE
  (if (`self.SmokeOnOff?`)
    (if (> (`ChaosVehicleMovementComponent.GetForwardSpeed` (`self.VehicleMovementComponent`)) 150.0)
      (`SceneComponent.SetVisibility` _smoke true false)
      (else
        (`SceneComponent.SetVisibility` _smoke false false)))))

(fn `Camera_Input`
  (`SceneComponent.K2_AddRelativeRotation` (`self.MainSpringArm`) (`KismetMathLibrary.MakeRotator` 0.0 (`self.GetInputAxisValue`) (`self.GetInputAxisValue`)) false false))

(fn `Car_Sound`
  (`AudioComponent.SetFloatParameter` (`self.EngineSound`) "RPM" (`ChaosVehicleMovementComponent.GetForwardSpeed` (`self.VehicleMovementComponent`))))

(fn `FlipCar`
  (bind (_returnvalue_x _returnvalue_y _returnvalue_z) (`KismetMathLibrary.BreakVector` (`self.K2_GetActorLocation`)))
  (bind (_returnvalue_roll _returnvalue_pitch _returnvalue_yaw) (`KismetMathLibrary.BreakRotator` (`self.K2_GetActorRotation`)))
  (`self.K2_SetActorTransform` (`KismetMathLibrary.MakeTransform` (`KismetMathLibrary.MakeVector` _returnvalue_x _returnvalue_y (+ _returnvalue_z 200.0)) (`KismetMathLibrary.MakeRotator` 0.0 0.0 _returnvalue_yaw)) false true))

(fn `FuelFinish`
  (`ChaosVehicleMovementComponent.SetThrottleInput` (`self.VehicleMovementComponent`) 0.0)
  (`AudioComponent.Stop` (`self.EngineSound`)))

(fn `FuelSystem`
  ;[0 0 0] FUEL SYSTEM
  (if (`self.FuelSystemOn-Off?`)
    (`|ExecutionSequence`
      (:`then_0`
        (if (> (`ChaosVehicleMovementComponent.GetForwardSpeed` (`self.VehicleMovementComponent`)) 50.0)
          (set `self.Fuel` (- (`self.Fuel`) (`self.FuelConsumptionRate`)) :!label _label)
          (if (< (`self.Fuel`) 1.0)
            (set `self.FuelFinish?` true)
            (else
              (set `self.FuelFinish?` false)))))
      (:`then_1`
        (if (< (`ChaosVehicleMovementComponent.GetForwardSpeed` (`self.VehicleMovementComponent`)) -50.0)
          (goto _label))))))

(fn `InteriorCamera_Input`
  (`SceneComponent.K2_AddRelativeRotation` (`self.InteriorSpringArm`) (`KismetMathLibrary.MakeRotator` 0.0 (`self.GetInputAxisValue`) (`self.GetInputAxisValue`)) false false))

(fn `ReverseLights`
  (bind _reverselightleft (`self.ReverseLightLeft`))
  (if (< (`ChaosVehicleMovementComponent.GetForwardSpeed` (`self.VehicleMovementComponent`)) -40.0)
    (`SceneComponent.SetVisibility` _reverselightleft true false)
    (`SceneComponent.SetVisibility` (`self.ReverseLightRight`) true false)
    (`SceneComponent.SetVisibility` (`self.REAR LIGHTS`) true false)
    (else
      (`SceneComponent.SetVisibility` _reverselightleft false false)
      (`SceneComponent.SetVisibility` (`self.ReverseLightRight`) false false)
      (`SceneComponent.SetVisibility` (`self.REAR LIGHTS`) false false))))

(fn `SteeringWheelRotation`
  (params (DeltaSec :type "Float (double-precision)"))
  (bind _steeringwheel (`self.SteeringWheel`))
  (bind _aschaos_wheeled_vehicle_movement_component (cast `ChaosWheeledVehicleMovementComponent` (`self.VehicleMovementComponent`)))
  (`|ExecutionSequence`
    (:`then_0`
      (bind _wheels (`ChaosWheeledVehicleMovementComponent.Wheels` _aschaos_wheeled_vehicle_movement_component))
      (bind _returnvalue (`ChaosVehicleWheel.GetSteerAngle` (`|GetArrayItem` _wheels)))
      (bind _returnvalue_2 (`ChaosVehicleWheel.GetSteerAngle` (`|GetArrayItem` _wheels 1)))
      (bind _returnvalue_3 (`KismetMathLibrary.SelectFloat` _returnvalue _returnvalue_2 (>= (`KismetMathLibrary.Abs` _returnvalue) (`KismetMathLibrary.Abs` _returnvalue_2))))
      (`SceneComponent.K2_SetRelativeRotation` _steeringwheel (`KismetMathLibrary.MakeRotator` _returnvalue_3 -30.0) false false))
    (:`then_1`
      (`SceneComponent.K2_SetRelativeRotation` _steeringwheel (`KismetMathLibrary.MakeRotator` _returnvalue_3 -30.0) false false))))

(fn `UserConstructionScript`)

(fn `Vehicle_Inputs`
  (bind _vehiclemovementcomponent (`self.VehicleMovementComponent`))
  ;[0 0 0 1 30] VEHICLE INPUTS
  (`ChaosVehicleMovementComponent.SetBrakeInput` _vehiclemovementcomponent (`self.GetInputAxisValue`))
  (`ChaosVehicleMovementComponent.SetSteeringInput` _vehiclemovementcomponent (`self.GetInputAxisValue`))
  (`ChaosVehicleMovementComponent.SetThrottleInput` _vehiclemovementcomponent (`self.GetInputAxisValue`))
  (`ChaosVehicleMovementComponent.GetBrakeInput` (`self.VehicleMovementComponent`)))