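; Blueprint actor that emits a Niagara sand effect from a configurable skeletal mesh.
; The construction script assigns the mesh and binds its component to the camera-facing sand system as a user variable, noting that the mesh needs CPU access.
; It also passes wind direction, wind speed and spawn scale to Niagara and rotates a direction component to match the wind vector.
; The event graph holds no active logic.
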(fn `UserConstructionScript`
  (bind _skeletalmesh (`self.SkeletalMesh`))
  ;[0 0 0] Add CPU Access to Skeletal Mesh
  (`SkinnedMeshComponent.SetSkinnedAssetAndUpdate` _skeletalmesh (`self.Skeletal_Mesh`) false)
  (`NiagaraFunctionLibrary.OverrideSystemUserVariableSkeletalMeshComponent` (`self.NS_Sand_From_Skeletal_Mesh_Camera_Face`) "SkeletalMesh" _skeletalmesh)
  (`FXSystemComponent.SetVectorParameter` (`self.NS_Sand_From_Skeletal_Mesh_Camera_Face`) "WindDirection" (`self.Wind_Direction`))
  (`FXSystemComponent.SetFloatParameter` (`self.NS_Sand_From_Skeletal_Mesh_Camera_Face`) "WindSpeed" (`self.Wind_Speed`))
  (`FXSystemComponent.SetFloatParameter` (`self.NS_Sand_From_Skeletal_Mesh_Camera_Face`) "Scale Spawn Amount" (`self.Scale_Spawn_Amount`))
  (`SceneComponent.K2_SetWorldRotation` (`self.WindDirection`) (`KismetMathLibrary.MakeRotFromX` (`self.Wind_Direction`)) false false))