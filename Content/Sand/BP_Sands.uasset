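; Deformable sand actor built on a dynamic mesh with Geometry Script, seeded from a debris static mesh, that supports digging and depositing.
; Erase boolean-subtracts a sphere, fills holes and smooths the affected vertices.
; Put queues locations; Tick turns the first few into cone-like piles using downward traces around a raised top, then clears the queue.
; Pile meshes are merged before one union into the main mesh, followed by a puff effect.
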(event Events|EventOnRebuildGeneratedMesh
  (params (TargetMesh :type Dynamic%20Mesh%20Object%20Reference))
  (bind _dynamicmeshcomponent (Variables|DynamicMeshActor|GetDynamicMeshComponent))
  ;[0.15 0.15 0.15 0.5] Создание первичной кучи песка
  (bind _output_get (Variables|Default|SetMainDM TargetMesh))
  (bind _returnvalue (GeometryScript|MeshEdits|AppendMesh :TargetMesh _output_get :AppendMesh (Variables|Default|GetPileDM) :Debug 0))
  (Class|GeometryScriptLibraryMeshRepairFunctions|FillAllMeshHoles :TargetMesh _returnvalue :Debug 0)
  (Class|DynamicMeshComponent|EnableComplexasSimpleCollision _dynamicmeshcomponent)
  (Collision|SetCollisionObjectType _dynamicmeshcomponent "ECC_WorldDynamic"))

(event EventBeginPlay
  (|CallParentFunction))

(event EventTick
  (params (DeltaSeconds :type Float%20%28single-precision%29))
  (|CallParentFunction DeltaSeconds)
  (if (Utilities|Array|IsNotEmpty (Variables|Default|GetFallenSandLocations))
    (Variables|Default|SetIgnore%20Actors (CallFunction|GetIgnoreActors))
    (bind _lastsandlocation (CallFunction|SpawnNewPiles))
    (Niagara|SpawnSystematLocation "/Game/Sand/VFX/VFX/LitSandPuff/NS_SandPuff_Medium.NS_SandPuff_Medium" (- _lastsandlocation "0.000000,0.000000,10.000000"))))

(event EventErase
  (params (Location :type Vector :default "0, 0, 0"))
  (CallFunction|EraseMeshfromLocation Location))

(event EventPut
  (params (Location :type Vector :default "0, 0, 0"))
  (Utilities|Array|Add (Variables|Default|GetFallenSandLocations) Location))

(fn ConstructionScript
  (Utilities|FlowControl|Sequence
    (:then_0
      (bind _returnvalue (DynamicMeshActor|AllocateComputeMesh))
      (bind _returnvalue_2 (Class|GeometryScriptLibraryStaticMeshFunctions|CopyMeshfromStaticMeshV2 :FromStaticMeshAsset "/Engine/BasicShapes/Sphere.Sphere" :ToDynamicMesh _returnvalue :Debug 0)
        (:Success
          (Variables|Default|SetSphereDM _returnvalue_2))))
    (:then_1
      (bind _returnvalue_3 (DynamicMeshActor|AllocateComputeMesh))
      (bind _returnvalue_4 (GeometryScript|StaticMesh|CopyMeshFromStaticMesh :FromStaticMeshAsset "/Game/Sand/Assets/SM_Debris_Origin.SM_Debris_Origin" :ToDynamicMesh _returnvalue_3 :Debug 0)
        (:Success
          (Variables|Default|SetPileDM _returnvalue_4))))))

(fn EraseMeshfromLocation
  (params (Tool%20%20Location :type Vector))
  (LocalVariables|SetErasingPoint (Math|Transform|InverseTransformLocation (Transformation|GetWorldTransform (Variables|DynamicMeshActor|GetDynamicMeshComponent)) Tool%20%20Location))
  (bind _returnvalue (GeometryScript|Booleans|ApplyMeshBoolean :TargetMesh (Variables|Default|GetMainDM) :ToolMesh (Variables|Default|GetSphereDM) :ToolTransform (Math|Transform|MakeTransform (LocalVariables|GetErasingPoint) "0, 0, 0" (LocalVariables|GetToolScale)) :Operation "Subtract" :Debug 0))
  (bind _returnvalue_2 (Class|GeometryScriptLibraryMeshRepairFunctions|FillAllMeshHoles :TargetMesh _returnvalue :Debug 0))
  (bind (_selection _returnvalue_3) (Class|GeometryScriptLibraryMeshSelectionFunctions|SelectMeshElementsInsideMesh _returnvalue_2 (Variables|Default|GetSphereDM) (Math|Transform|MakeTransform (LocalVariables|GetErasingPoint) "0, 0, 0" (+ (LocalVariables|GetToolScale) "0.200000,0.200000,0.200000")) "Vertices" false 0.0 0.5))
  (Class|GeometryScriptLibraryMeshDeformFunctions|ApplyIterativeSmoothingtoMesh _returnvalue_3 _selection (Utilities|Struct|MakeGeometryScriptIterativeMeshSmoothingOptions 10 0.1 "FullMeshSelection") 0))

(fn ConvertLocation
  (params (Location :type Vector))
  (return (Math|Transform|InverseTransformLocation (Transformation|GetWorldTransform (Variables|DynamicMeshActor|GetDynamicMeshComponent)) Location)))

(fn GenerateVerticlesAroundPileTop
  (params (InputPin :type Vector) (Radius :type Float%20%28double-precision%29) (PileHeight :type Float%20%28double-precision%29))
  (bind (_success _out_hit_location) (CallFunction|TracefromUptoDown InputPin))
  (if _success
    (bind _output_get (LocalVariables|SetPileTop (Math|Vector|MakeVector (.x _out_hit_location) (.y _out_hit_location) (+ (.z _out_hit_location) PileHeight))))
    (Utilities|Array|Add (LocalVariables|GetPointsAround) _output_get)
    (Utilities|FlowControl|Sequence
      (:then_0
        (CallFunction|DrawDebugLocation _output_get 5.0 "(R=0.000000,G=0.051529,B=1.000000,A=1.000000)"))
      (:then_1
        (for _index (range 1 (Variables|Default|GetVerticlesCount))
          (bind _output_get_2 (LocalVariables|SetAngle (|((360/n)*i) (Math|Conversions|ToFloat(Integer) (Variables|Default|GetVerticlesCount)) (Math|Conversions|ToFloat(Integer) _index))))
          (bind _out_hit_location_2 (CallFunction|TracefromUptoDown (Math|Vector|MakeVector (+ (.x (LocalVariables|GetPileTop)) (* (Math|Trig|Cos(Degrees) _output_get_2) Radius)) (+ (.y (LocalVariables|GetPileTop)) (* Radius (Math|Trig|Sin(Degrees) _output_get_2))) (.z (LocalVariables|GetPileTop)))))
          (Utilities|Array|Add (LocalVariables|GetPointsAround) (- _out_hit_location_2 "0.000000,0.000000,10.000000")))
        (return (LocalVariables|GetPointsAround) (LocalVariables|GetPileTop))))))

(fn GeneratePileMesh
  (params (Verticles :type Array%20of%20Vectors) (AppendMesh :type Dynamic%20Mesh%20Object%20Reference))
  (for _array_element Verticles
    (Utilities|Array|Add (LocalVariables|GetConvertedVerticles) (CallFunction|ConvertLocation _array_element))
    (bind _vectorlist (GeometryScript|ListUtils|ConvertArraytoVectorList (LocalVariables|GetConvertedVerticles)))
    (bind _returnvalue (DynamicMeshActor|AllocateComputeMesh))
    (bind _returnvalue_2 (GeometryScript|MeshEdits|AddVerticestoMesh _returnvalue _vectorlist))
    (bind _trianglelist (Class|GeometryScriptLibraryListUtilityFunctions|ConvertArraytoTriangleList (Variables|Default|GetTriangle%20Tuple%20Array)))
    (bind _returnvalue_3 (Class|GeometryScriptLibraryMeshBasicEditFunctions|AddTrianglestoMesh _returnvalue_2 _trianglelist 0 false 0))
    (bind _returnvalue_4 (Class|GeometryScriptLibraryMeshNormalsFunctions|FlipNormals _returnvalue_3 0))
    (bind _returnvalue_5 (Class|GeometryScriptLibraryMeshNormalsFunctions|ComputeSplitNormals :TargetMesh _returnvalue_4 :Debug 0))
    (GeometryScript|Booleans|ApplyMeshBoolean :TargetMesh AppendMesh :ToolMesh _returnvalue_5 :Operation "Union" :Debug 0)
    (Class|DynamicMeshActor|ReleaseComputeMesh _returnvalue_5)))

(fn DrawDebugLocation
  (params (Location :type Vector) (Size :type Float%20%28single-precision%29) (PointColor :type Linear%20Color%20Structure))
  (if (Variables|Default|GetbDebug)
    (Rendering|Debug|DrawDebugPoint Location Size PointColor 1e+02)))

(fn SpawnNewPiles
  (bind _fallensandlocations (Variables|Default|GetFallenSandLocations))
  (bind _returnvalue (DynamicMeshActor|AllocateComputeMesh))
  (LocalVariables|SetNewPileMesh _returnvalue)
  (for (_array_element _array_index) _fallensandlocations
    (if (<= _array_index 10)
      (bind (_output_get _piletoplocation) (CallFunction|GenerateVerticlesAroundPileTop _array_element 6e+01 2e+01))
      (CallFunction|GeneratePileMesh _output_get (LocalVariables|GetNewPileMesh))
      (LocalVariables|SetSandLocation _piletoplocation)))
  (Utilities|Array|Clear _fallensandlocations)
  (GeometryScript|Booleans|ApplyMeshBoolean :TargetMesh (Variables|Default|GetMainDM) :ToolMesh (LocalVariables|GetNewPileMesh) :Operation "Union" :Debug 0)
  (Class|DynamicMeshActor|ReleaseComputeMesh (LocalVariables|GetNewPileMesh))
  (return (LocalVariables|GetSandLocation)))

(fn GetIgnoreActors
  (for _array_element (Variables|Default|GetActorsToCollisionIgnore)
    (bind _returnvalue (Actor|GetActorOfClass _array_element))
    (Utilities|Array|Add (LocalVariables|GetActors) _returnvalue))
  (return (LocalVariables|GetActors)))

(fn TracefromUptoDown
  (params (InVec :type Vector))
  (bind (_x _y) (Math|Vector|BreakVector InVec))
  (bind _returnvalue (+ InVec "0.000000,0.000000,100.000000"))
  (bind _outhit (Collision|LineTraceByChannel _returnvalue (Math|Vector|MakeVector _x _y -1e+02) "TraceTypeQuery1" false (Variables|Default|GetIgnore%20Actors) "None" false))
  (if (.bblockinghit _outhit)
    (CallFunction|DrawDebugLocation (.location _outhit) 5.0 "(R=0.000000,G=1.000000,B=0.156678,A=1.000000)")
    (return true (.location _outhit))
    (else
      (Development|PrintString (Utilities|GetDisplayName (.hitactor _outhit)))
      (CallFunction|DrawDebugLocation _returnvalue 2e+01 "(R=1.000000,G=0.048188,B=0.000000,A=1.000000)")
      (return false "0, 0, 0"))))